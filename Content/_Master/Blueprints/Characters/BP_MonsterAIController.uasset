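; BP_MonsterAIController is the AI controller for a roaming monster that detects the player by sight.
; On BeginPlay it runs the BT_RoamingMonster behavior tree and caches its blackboard.
; AI Perception sight updates for the player character set the TargetActor key to the player when sensed, or clear it to null when sight is lost.
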(event OnTargetPerceptionUpdated(AIPerception)
  (params (Actor :type Actor%20Object%20Reference) (Stimulus :type AI%20Stimulus%20Structure))
  (bind _returnvalue (Game|GetPlayerCharacter 0))
  (bind _returnvalue_2 (Class|AIPerceptionSystem|GetSenseClassforStimulus Stimulus))
  (if (and (== _returnvalue_2 "/Script/AIModule.AISense_Sight") (== Actor _returnvalue))
    (AI|Components|Blackboard|SetValueasObject (Variables|Default|GetAIBlackboard) (Utilities|Name|MakeLiteralName "TargetActor") (Utilities|SelectObject _returnvalue 0 (.bSuccessfullySensed (Utilities|Struct|BreakAIStimulus Stimulus))))))

(event EventBeginPlay
  (AI|RunBehaviorTree "/Game/_Master/Blueprints/AI/Behavior/BT_RoamingMonster.BT_RoamingMonster")
  (Variables|Default|SetAIBlackboard (AI|GetBlackboard 0)))

(event EventTick
  (params (DeltaSeconds :type Float%20%28single-precision%29)))

(fn ConstructionScript)